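; BP_Bounding_Box is a side-on follow camera actor that becomes the player controller's view target and tracks the player character.
; Each Tick moves it along X and Z only when the character leaves a dead zone, keeping Y at a set offset.
; A nonzero FixedXValue locks X, while FixedZValue only affects construction, as its GetZ branch is unwired.
; The construction script pre-positions and yaws it toward a valid ActorToFollow.
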(event EventBeginPlay
  (Variables|Default|SetActor%20to%20follow (Game|GetPlayerCharacter 0))
  (Game|Player|SetViewTargetwithBlend (Game|GetPlayerController 0) self 0.0 "VTBlend_Linear" 0.0 false))

(event EventTick
  (params (DeltaSeconds :type Float%20%28single-precision%29))
  (bind _new_x (CallFunction|GetX))
  (Variables|Default|SetCameraX _new_x)
  (bind _new_z (CallFunction|GetZ))
  (Variables|Default|SetCameraZ _new_z)
  (Transformation|SetActorLocation (Math|Vector|MakeVector (Variables|Default|GetCameraX) (Variables|Default|GetYoffset) (Variables|Default|GetCameraZ)) false false))

(fn ConstructionScript
  (bind _actor_to_follow (Variables|Default|GetActor%20to%20follow))
  (bind _returnvalue (Transformation|GetActorLocation _actor_to_follow))
  (Utilities|IsValid _actor_to_follow
    (:Is%20Valid
      (bind _output_get (Variables|Default|SetCameraX (.x _returnvalue)))
      (if (!= (Variables|Default|GetFixed%20Z%20Value) 0.0)
        (Variables|Default|SetCameraZ (Variables|Default|GetFixed%20Z%20Value))
        (else
          (bind _output_get_2 (Variables|Default|SetCameraZ (+ (.z _returnvalue) (Variables|Default|GetZDeadZone))))))
      (Transformation|SetActorLocation (Math|Vector|MakeVector _output_get (Variables|Default|GetYoffset) _output_get_2) false false)
      (Transformation|SetActorRotation (Math|Rotator|MakeRotator 0.0 0.0 (.yaw (Math|Rotator|FindLookatRotation (Transformation|GetActorLocation) (Transformation|GetActorLocation (Variables|Default|GetActor%20to%20follow)))))))))

(fn GetX
  (bind _actor_to_follow (Variables|Default|GetActor%20to%20follow))
  (bind _xdeadzone (Variables|Default|GetXDeadzone))
  (bind _actor_to_follow_2 (Variables|Default|GetActor%20to%20follow))
  (bind _xdeadzone_2 (Variables|Default|GetXDeadzone))
  (bind _returnvalue (Transformation|GetActorLocation _actor_to_follow))
  (bind _returnvalue_2 (Transformation|GetActorLocation _actor_to_follow_2))
  (bind _returnvalue_3 (- (.x _returnvalue_2) _xdeadzone_2))
  (bind _returnvalue_4 (+ (.x _returnvalue) _xdeadzone))
  (if (!= (Variables|Default|GetFixed%20X%20Value) 0.0)
    (return (Variables|Default|GetFixed%20X%20Value))
    (elif (> _returnvalue_3 (.x (Transformation|GetActorLocation)))
      (return _returnvalue_3)
      (elif (< _returnvalue_4 (.x (Transformation|GetActorLocation)))
        (return _returnvalue_4)
        (else
          (return (Variables|Default|GetCameraX)))))))

(fn GetZ
  (bind _actor_to_follow (Variables|Default|GetActor%20to%20follow))
  (bind _actor_to_follow_2 (Variables|Default|GetActor%20to%20follow))
  (bind _zdeadzone (Variables|Default|GetZDeadZone))
  (bind _zdeadzone_2 (Variables|Default|GetZDeadZone))
  (bind _returnvalue (Transformation|GetActorLocation _actor_to_follow))
  (bind _returnvalue_2 (Transformation|GetActorLocation _actor_to_follow_2))
  (bind _returnvalue_3 (- (.z _returnvalue_2) _zdeadzone))
  (bind _returnvalue_4 (+ (.z _returnvalue) _zdeadzone_2))
  ;[1 1 1] Camera Dead Zone on Z
  (if (> _returnvalue_3 (.z (Transformation|GetActorLocation)))
    (return _returnvalue_3)
    (elif (< _returnvalue_4 (.z (Transformation|GetActorLocation)))
      (return _returnvalue_4)
      (else
        (return (Variables|Default|GetCameraZ))))))