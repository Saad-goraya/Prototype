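; BP_EnemySimple is a basic enemy that homes in on the player and deals contact damage.
; On BeginPlay it sets the player's StaticMesh as the ProjectileMovement homing target.
; When its Box overlaps a BP_Player_Base, it applies fixed damage to that player and destroys itself.
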(event OnComponentBeginOverlap(Box)
  (params (OverlappedComponent :type Primitive%20Component%20Object%20Reference) (OtherActor :type Actor%20Object%20Reference) (OtherComp :type Primitive%20Component%20Object%20Reference) (OtherBodyIndex :type Integer) (bFromSweep :type Boolean) (SweepResult :type Hit%20Result%20Structure%20%28by%20ref%29))
  (bind _asbp_player_base (Utilities|Casting|CastToBP_Player_Base OtherActor))
  (Variables|Default|SetAs%20BP%20Player%20Base _asbp_player_base)
  (Game|Damage|ApplyDamage (Variables|Default|GetAs%20BP%20Player%20Base) 2e+01 0 0)
  (Actor|DestroyActor))

(event EventBeginPlay
  (Variables|/Script/Engine.ProjectileMovementComponent|SetHomingTargetComponent (Variables|Default|GetProjectileMovement) (Variables|/Game/Assets/G_Prototype/Character/BP_Player_Base.BP_Player_Base_C|GetStaticMesh (.AsBP%20Player%20Base (Utilities|Casting|CastToBP_Player_Base (Game|Player|GetPlayerPawn 0))))))

(event Collision|EventActorBeginOverlap
  (params (OtherActor :type Actor%20Object%20Reference)))

(event EventTick
  (params (DeltaSeconds :type Float%20%28single-precision%29)))

(fn ConstructionScript)