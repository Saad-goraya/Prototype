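; Base player character for a flying ship with health, regenerating on a looping timer, and a pausing game-over screen at zero health.
; BeginPlay sets up the HUD, cursor and Enhanced Input, whose movement actions switch to Flying mode and steer the ship.
; Tick applies a constant Z-axis impulse and interpolates max fly speed toward boost while Left Shift is held.
; Two fire actions spawn projectiles: one unguided, one homing on the component under the cursor.
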(event Custom|Healing
  ;[1 1 1] Damage and healing
  (if (== (Variables|Default|GetPlayer%20health) 1e+02)
    (Development|PrintString ".")
    (else
      (Variables|Default|SetPlayer%20health (+ (Variables|Default|GetPlayer%20health) 1e+01)))))

(event Input|EnhancedActionEvents|EnhancedInputActionIA_Shoot
  (params (ActionValue :type Boolean) (ElapsedSeconds :type Float%20%28double-precision%29) (TriggeredSeconds :type Float%20%28double-precision%29) (InputAction :type Input%20Action%20Object%20Reference :default "/Game/Assets/G_Prototype/Character/Inputs/IA_Shoot.IA_Shoot"))
  (bind _returnvalue (Transformation|GetActorLocation))
  ;[1 1 1] Projectiles
  (:Started
    (bind _returnvalue_2 (Game|SpawnActorfromClass "/Game/Assets/G_Prototype/Character/BP_Fire2.BP_Fire2_C" (Math|Transform|MakeTransform (Math|Vector|MakeVector (+ (.x _returnvalue) 2e+02) (.y _returnvalue) (+ (.z _returnvalue) -1e+02)) (Transformation|GetActorRotation) "1.000000,1.000000,1.000000") "Undefined" "MultiplyWithRoot" 0 0))
    (Variables|/Script/Engine.ProjectileMovementComponent|SetHomingTargetComponent (Variables|/Game/Assets/G_Prototype/Character/BP_Fire2.BP_Fire2_C|GetProjectileMovement _returnvalue_2) 0)))

(event Input|EnhancedActionEvents|EnhancedInputActionIA_Shoot2
  (params (ActionValue :type Boolean) (ElapsedSeconds :type Float%20%28double-precision%29) (TriggeredSeconds :type Float%20%28double-precision%29) (InputAction :type Input%20Action%20Object%20Reference :default "/Game/Assets/G_Prototype/Character/Inputs/IA_Shoot2.IA_Shoot2"))
  (bind _returnvalue (Transformation|GetActorLocation))
  ;[1 1 1] Projectiles
  (:Started
    (bind _returnvalue_2 (Game|SpawnActorfromClass "/Game/Assets/G_Prototype/Character/BP_Fire.BP_Fire_C" (Math|Transform|MakeTransform (Math|Vector|MakeVector (.x _returnvalue) (.y _returnvalue) (+ (.z _returnvalue) -2e+02)) (Transformation|GetActorRotation) "1.000000,1.000000,1.000000") "Undefined" "MultiplyWithRoot" 0 0))
    (Variables|/Script/Engine.ProjectileMovementComponent|SetHomingTargetComponent (Variables|/Game/Assets/G_Prototype/Character/BP_Fire.BP_Fire_C|GetProjectileMovement _returnvalue_2) (.HitComponent (Collision|BreakHitResult (.HitResult (Game|Player|GetHitResultUnderCursorbyChannel (Game|GetPlayerController 0) "TraceTypeQuery1" true)))))))

(event Input|EnhancedActionEvents|EnhancedInputActionIA_Right_Left
  (params (ActionValue :type Float%20%28double-precision%29) (ElapsedSeconds :type Float%20%28double-precision%29) (TriggeredSeconds :type Float%20%28double-precision%29) (InputAction :type Input%20Action%20Object%20Reference :default "/Game/Assets/G_Prototype/Character/Inputs/IA_Right_Left.IA_Right_Left"))
  ;[1 1 1] Right/Left/Up/Down Movement
  (:Triggered
    (Pawn|Input|AddMovementInput (Math|Vector|GetForwardVector (Math|Rotator|MakeRotator 0.0 (.pitch (Pawn|GetControlRotation :!class /Script/Engine.Pawn)) 0.0)) ActionValue false))
  (:Started
    (Pawn|Components|CharacterMovement|SetMovementMode (Variables|Character|GetCharacterMovement) "MOVE_Flying" 0)))

(event Input|EnhancedActionEvents|EnhancedInputActionIA_Up_Down
  (params (ActionValue :type Float%20%28double-precision%29) (ElapsedSeconds :type Float%20%28double-precision%29) (TriggeredSeconds :type Float%20%28double-precision%29) (InputAction :type Input%20Action%20Object%20Reference :default "/Game/Assets/G_Prototype/Character/Inputs/IA_Up_Down.IA_Up_Down"))
  ;[1 1 1] Right/Left/Up/Down Movement
  (:Triggered
    (if (Class|NavMovementComponent|IsFlying (Variables|Character|GetCharacterMovement))
      (Pawn|Input|AddMovementInput (Transformation|GetActorUpVector (Pawn|GetController)) ActionValue false)))
  (:Started
    (Pawn|Components|CharacterMovement|SetMovementMode (Variables|Character|GetCharacterMovement) "MOVE_Flying" 0)))

(event EventBeginPlay
  (bind _returnvalue (Game|GetPlayerController 0))
  ;[1 1 1] Widget
  (Utilities|FlowControl|Sequence
    (:then_0
      (Input|SetInputModeGameOnly _returnvalue false)
      (bind _returnvalue_2 (UserInterface|CreateWidget "/Game/Assets/G_Prototype/UI/WBP_Main.WBP_Main_C"))
      (UserInterface|Viewport|AddtoViewport _returnvalue_2 0)
      (Variables|/Script/Engine.PlayerController|SetbShowMouseCursor _returnvalue true)
      (Class|GameplayStatics|SetViewportMouseCaptureMode "CapturePermanently_IncludingInitialMouseDown")
      ;[1 1 1] Enhanced Input
      (bind _asplayer_controller (Utilities|Casting|CastToPlayerController (Game|GetPlayerController 0)))
      (Utilities|IsValid (PlayerController|LocalPlayerSubsystems|GetEnhancedInputLocalPlayerSubsystem _asplayer_controller)
        (:Is%20Valid
          (Input|AddMappingContext (PlayerController|LocalPlayerSubsystems|GetEnhancedInputLocalPlayerSubsystem _asplayer_controller) "/Game/Assets/G_Prototype/Character/Inputs/IMC_Main.IMC_Main" 0 "(bIgnoreAllPressedKeysUntilRelease=True,bForceImmediately=False,bNotifyUserSettings=False)"))))
    (:then_1
      ;[1 1 1] Damage and healing
      (Utilities|Time|SetTimerbyEvent (delegate Custom|Healing) 1.0 true))))

(event Game|Damage|EventAnyDamage
  (params (Damage :type Float%20%28single-precision%29) (DamageType :type Damage%20Type%20Object%20Reference) (InstigatedBy :type Controller%20Object%20Reference) (DamageCauser :type Actor%20Object%20Reference))
  ;[1 1 1] Damage and healing
  (Variables|Default|SetPlayer%20health (- (Variables|Default|GetPlayer%20health) Damage))
  ;;[1 1 1] Game Over UI
  (if (<= (Variables|Default|GetPlayer%20health) 0.0)
    (bind _returnvalue (UserInterface|CreateWidget "/Game/Assets/G_Prototype/UI/WBP_GameOver.WBP_GameOver_C"))
    (UserInterface|Viewport|AddtoViewport _returnvalue 0)
    (Game|SetGamePaused true)))

(event EventTick
  (params (DeltaSeconds :type Float%20%28single-precision%29))
  ;[1 1 1] Ship Default Speed
  (Utilities|FlowControl|Sequence
    (:then_0
      (Physics|AddImpulse (Variables|Character|GetCharacterMovement) (Math|Vector|MakeVector 0.0 0.0 (Variables|Default|GetShipDefaultSpeed)) true))
    (:then_1
      ;[1 1 1] Gradual Speed Boost
      (CallFunction|GradualSpeed))))

(event Input|KeyboardEvents|LeftShift
  (params (Key :type Key%20Structure :default "None"))
  ;[1 1 1] Gradual Speed Boost
  (:Pressed
    (Variables|Default|SetFull%20Speed true))
  (:Released
    (Variables|Default|SetFull%20Speed false)))

(fn ConstructionScript)

(fn GradualSpeed
  (bind _charactermovement (Variables|Character|GetCharacterMovement))
  (bind _charactermovement_2 (Variables|Character|GetCharacterMovement))
  (if (Variables|Default|GetFull%20Speed)
    (Variables|/Script/Engine.CharacterMovementComponent|SetMaxFlySpeed _charactermovement (Math|Interpolation|FInterpTo (Variables|/Script/Engine.CharacterMovementComponent|GetMaxFlySpeed _charactermovement) (Variables|Default|GetBoost%20Speed) (Utilities|Time|GetWorldDeltaSeconds) (Variables|Default|GetSpeedTime)))
    (else
      (Variables|/Script/Engine.CharacterMovementComponent|SetMaxFlySpeed _charactermovement_2 (Math|Interpolation|FInterpTo (Variables|/Script/Engine.CharacterMovementComponent|GetMaxFlySpeed _charactermovement_2) (Variables|Default|GetNormal%20Speed) (Utilities|Time|GetWorldDeltaSeconds) (Variables|Default|GetSpeedTime))))))