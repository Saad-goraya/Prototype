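; BP_Fire2 is an explosive actor, apparently a fire attack, that detonates on impact and harms enemies.
; A Box hit fires a radial force impulse, spawns an explosion emitter at the hit location and destroys the actor.
; Separately, a Sphere overlap applies damage to BP_Drone actors and destroys BP_EnemySimple actors outright.
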(event OnComponentBeginOverlap(Sphere)
  (params (OverlappedComponent :type Primitive%20Component%20Object%20Reference) (OtherActor :type Actor%20Object%20Reference) (OtherComp :type Primitive%20Component%20Object%20Reference) (OtherBodyIndex :type Integer) (bFromSweep :type Boolean) (SweepResult :type Hit%20Result%20Structure%20%28by%20ref%29))
  (Utilities|FlowControl|Sequence
    (:then_0
      (bind _asbp_drone (Utilities|Casting|CastToBP_Drone OtherActor))
      (Variables|Default|SetAs%20BP%20Drone _asbp_drone)
      (Game|Damage|ApplyDamage (Variables|Default|GetAs%20BP%20Drone) 1e+01 0 0))
    (:then_1
      (bind _asbp_enemy_simple (Utilities|Casting|CastToBP_EnemySimple OtherActor))
      (Actor|DestroyActor _asbp_enemy_simple))))

(event OnComponentHit(Box)
  (params (HitComponent :type Primitive%20Component%20Object%20Reference) (OtherActor :type Actor%20Object%20Reference) (OtherComp :type Primitive%20Component%20Object%20Reference) (NormalImpulse :type Vector :default "0, 0, 0") (Hit :type Hit%20Result%20Structure%20%28by%20ref%29))
  (Class|RadialForceComponent|FireImpulse (Variables|Default|GetRadialForce))
  (Effects|SpawnEmitteratLocation "/Game/StarterContent/Particles/P_Explosion.P_Explosion" (.Location (Collision|BreakHitResult Hit)))
  (Actor|DestroyActor))

(event EventBeginPlay)

(event Collision|EventActorBeginOverlap
  (params (OtherActor :type Actor%20Object%20Reference)))

(fn ConstructionScript)